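; AC_Detector is a stealth component that decides which detectable objects its owning actor can currently see.
; DetectableEntered and DetectableExited maintain the tracked candidates, and each tick it line-traces on a vision channel from a rotated owner offset to each candidate's view points.
; A candidate with enough unblocked points counts as spotted.
; Changes to the spotted state notify the owner through the BI_DetectorOwner interface.
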(event `self.ReceiveTick`
  (params (DeltaSeconds :type "Float (single-precision)"))
  (bind _trackeddetectables (`self.TrackedDetectables`))
  (bind _spotteddetectables (`self.SpottedDetectables`))
  (if (> (`KismetArrayLibrary.Array_Length` _trackeddetectables) 0)
    (for _array_element _trackeddetectables
      ;[0.8249 0.2874 1] Determine visibility of object
      (bind _viewpoints (`/Game/Assets/Actors/Components/Stealth/BI_Detectable.GetViewPoints` _array_element))
      (set `self.ViewedPoints` 0)
      (for _array_element_2 _viewpoints
        (bind _returnvalue (`self.GetViewPosition`))
        ;;[0.4736 1 0.2071] Detected if not colliding with view blockers
        (bind (_outhit _returnvalue_2) (`KismetSystemLibrary.LineTraceSingle` _returnvalue _array_element_2 (`self.VisionChannel`) true))
        (if (not _returnvalue_2)
          (set `self.ViewedPoints` (+ (`self.ViewedPoints`) 1))))
      (if (>= (`self.ViewedPoints`) (`self.ViewPointDetectionCount`))
        (bind _returnvalue_3 (`KismetArrayLibrary.Array_Find` _spotteddetectables _array_element))
        (bind _returnvalue_4 (== _returnvalue_3 -1))
        ;;[0 1 0.06384] Newly Detected
        (if _returnvalue_4
          (`KismetArrayLibrary.Array_Add` _spotteddetectables _array_element)
          (bind _asbi_detector_owner (cast `/Game/Assets/Actors/Components/Stealth/BI_DetectorOwner` (`self.GetOwner`)))
          (`/Game/Assets/Actors/Components/Stealth/BI_DetectorOwner.DetectableEnteredView` _asbi_detector_owner _array_element))
        (else
          ;;[1 0.08854 0.08854] Detected item hidden
          (if (not _returnvalue_4)
            (`KismetArrayLibrary.Array_Remove` _spotteddetectables _returnvalue_3)
            (bind _asbi_detector_owner_2 (cast `/Game/Assets/Actors/Components/Stealth/BI_DetectorOwner` (`self.GetOwner`)))
            (`/Game/Assets/Actors/Components/Stealth/BI_DetectorOwner.DetectableExitedView` _asbi_detector_owner_2 _array_element)))))))

(fn `DetectableEntered`
  (params (Detectable :type "/Game/Assets/Actors/Components/Stealth/BI_Detectable Interface"))
  (`KismetArrayLibrary.Array_Add` (`self.TrackedDetectables`) Detectable))

(fn `DetectableExited`
  (params (Detectable :type "/Game/Assets/Actors/Components/Stealth/BI_Detectable Interface"))
  (`KismetArrayLibrary.Array_RemoveItem` (`self.TrackedDetectables`) Detectable))

(fn `GetViewPosition`
  (returns (ReturnValue :type "Vector Structure"))
  (bind _returnvalue (`self.GetOwner`))
  (return (+ (`KismetMathLibrary.GreaterGreater_VectorRotator` (`self.ViewPositionOffset`) (`Actor.K2_GetActorRotation` _returnvalue)) (`Actor.K2_GetActorLocation` _returnvalue))))